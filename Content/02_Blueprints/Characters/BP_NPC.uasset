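; BP_NPC is a team-colored NPC character that shows its current health as text.
; The construction script sets the Body material from the Team enum, covering Red, Blue and Yellow.
; On BeginPlay, UpdateHealthUI copies the health value from the BPHealth component into the TextRender; nothing in this graph refreshes it afterward.
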(event `self.ReceiveBeginPlay`
  (`self.UpdateHealthUI`))

(fn `UpdateHealthUI`
  ; Update Health UI
  (`TextRenderComponent.K2_SetText` (`self.TextRender`) (`KismetTextLibrary.Conv_DoubleToText` (`/Game/02_Blueprints/Characters/BP_Health.Health` (`self.BP_Health`)) "HalfToEven")))

(fn `UserConstructionScript`
  (bind _body (`self.Body`))
  ; Sets Material from team
  (switch `/Game/04_Enums/E_Team` (`self.Team`)
    (:`NewEnumerator0`
      (`PrimitiveComponent.SetMaterial` _body 0 "/Game/05_Materials/M_Red.M_Red"))
    (:`NewEnumerator1`
      (`PrimitiveComponent.SetMaterial` _body 0 "/Game/05_Materials/M_Blue_2.M_Blue_2"))
    (:`NewEnumerator2`
      (`PrimitiveComponent.SetMaterial` _body 0 "/Game/05_Materials/M_Yellow.M_Yellow"))))